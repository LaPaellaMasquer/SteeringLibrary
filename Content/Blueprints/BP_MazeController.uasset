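; BP_MazeController is a player controller that turns mouse clicks on maze node actors into commands for the maze pawn.
; On BeginPlay it finds and caches the MazePawn in the level.
; Each click traces under the cursor on the Visibility channel and continues only if it hits a NodeGraph actor.
; Left click passes that node to the pawn's MoveToNode, and right click passes it to CreateCircuit.
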(event EventBeginPlay
  (bind _returnvalue (Actor|GetActorOfClass "/Script/Steering.MazePawn"))
  (Variables|Default|Setmazepawn _returnvalue))

(event EventTick
  (params (DeltaSeconds :type Float%20%28single-precision%29)))

(event Input|MouseEvents|RightMouseButton
  (params (Key :type Key%20Structure :default "None"))
  (:Pressed
    (bind _asnode_graph (Utilities|Casting|CastToNodeGraph (.HitActor (Collision|BreakHitResult (.HitResult (Game|Player|GetHitResultUnderCursorbyChannel "TraceTypeQuery1" true))))))
    (Class|MazePawn|CreateCircuit (Variables|Default|Getmazepawn) _asnode_graph)))

(event Input|MouseEvents|LeftMouseButton
  (params (Key :type Key%20Structure :default "None"))
  (:Pressed
    (bind _asnode_graph (Utilities|Casting|CastToNodeGraph (.HitActor (Collision|BreakHitResult (.HitResult (Game|Player|GetHitResultUnderCursorbyChannel "TraceTypeQuery1" true))))))
    (Class|MazePawn|MovetoNode (Variables|Default|Getmazepawn) _asnode_graph)))

(fn ConstructionScript)
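; An AI controller that switches a possessed SteerPawn between Circuit, One Way and Two Way movement modes.
; On BeginPlay it casts its controlled pawn to SteerPawn, caches it and starts Circuit mode.
; Three custom events call the matching function on the cached pawn and print the mode name to screen.
; The steering logic itself lives in SteerPawn.
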(event Custom|On%20Circuit
  (Class|SteerPawn|Circuit (Variables|Default|GetCiruitPawn))
  (Development|PrintString "Circuit"))

(event Custom|On%20Two%20Way
  (Class|SteerPawn|TwoWay (Variables|Default|GetCiruitPawn))
  (Development|PrintString "Two Way"))

(event Custom|On%20One%20Way
  (Class|SteerPawn|OneWay (Variables|Default|GetCiruitPawn))
  (Development|PrintString "One Way"))

(event EventBeginPlay
  (bind _assteer_pawn (Utilities|Casting|CastToSteerPawn (Pawn|GetControlledPawn)))
  (bind _output_get (Variables|Default|SetCiruitPawn _assteer_pawn))
  (Class|SteerPawn|Circuit _output_get))

(event EventTick
  (params (DeltaSeconds :type Float%20%28single-precision%29)))

(fn ConstructionScript)
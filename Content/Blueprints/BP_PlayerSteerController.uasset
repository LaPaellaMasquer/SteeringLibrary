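; Player controller for a steering-behaviour demo that drives a SteerPawn with mouse clicks and a CircuitPawn with keys.
; On BeginPlay it adds the UI, caches both pawns and starts the circuit.
; Cursor traces choose the behaviour: left-click pursues another pawn or seeks the point (arrival with Shift), right-click evades or flees, with points flattened to the pawn's height.
; A, Z and E switch between Circuit, One Way and Two Way.
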(event EventBeginPlay
  (bind _returnvalue (UserInterface|CreateWidget "/Game/Blueprints/UI.UI_C"))
  (bind _output_get (Variables|Default|SetUI _returnvalue))
  (UserInterface|Viewport|AddtoViewport _output_get 0)
  (bind _assteer_pawn (Utilities|Casting|CastToSteerPawn (Game|Player|GetPlayerPawn 0)))
  (Variables|Default|SetSteerPawn _assteer_pawn)
  (bind _returnvalue_2 (Actor|GetActorOfClass "/Game/Blueprints/CircuitPawn.CircuitPawn_C"))
  (bind _output_get_2 (Variables|Default|SetCircuitPawn _returnvalue_2))
  (Class|SteerPawn|Circuit _output_get_2))

(event EventTick
  (params (DeltaSeconds :type Float%20%28single-precision%29)))

(event Input|KeyboardEvents|A
  (params (Key :type Key%20Structure :default "None"))
  ;[1 1 1] CircuitPawn control
  (:Pressed
    (Class|SteerPawn|Circuit (Variables|Default|GetCircuitPawn))
    (Development|PrintString "Circuit")))

(event Input|KeyboardEvents|Z
  (params (Key :type Key%20Structure :default "None"))
  ;[1 1 1] CircuitPawn control
  (:Pressed
    (Class|SteerPawn|OneWay (Variables|Default|GetCircuitPawn))
    (Development|PrintString "One Way")))

(event Input|MouseEvents|LeftMouseButton
  (params (Key :type Key%20Structure :default "None"))
  (bind _hitresult (Game|Player|GetHitResultUnderCursorbyChannel "TraceTypeQuery1" true))
  (bind _steerpawn (Variables|Default|GetSteerPawn))
  (bind _steerpawn_2 (Variables|Default|GetSteerPawn))
  (bind _returnvalue (Transformation|GetActorLocation _steerpawn))
  (bind (_bblockinghit _binitialoverlap _time _distance _location _impactpoint _normal _impactnormal _physmat _hitactor) (Collision|BreakHitResult _hitresult))
  (bind _returnvalue_2 (Math|Vector|MakeVector (.x _location) (.y _location) (.z _returnvalue)))
  ;[1 1 1] Click Input Player Control
  (:Pressed
    (bind _aspawn (Utilities|Casting|CastToPawn _hitactor)
      (:then
        (if (!= _aspawn _steerpawn_2)
          (Class|SteerPawn|Pursuit _steerpawn_2 _aspawn)
          (Development|PrintString "Pursuit")
          (else
            (if (Variables|Default|GetisShiftPress) :!label _label
              (Class|SteerPawn|Arrival _steerpawn_2 _returnvalue_2)
              (Development|PrintString "Arrival")
              (else
                (Class|SteerPawn|Seek _steerpawn_2 _returnvalue_2)
                (Development|PrintString "Seek"))))))
      (:CastFailed
        (goto _label)))))

(event Input|MouseEvents|RightMouseButton
  (params (Key :type Key%20Structure :default "None"))
  (bind _hitresult (Game|Player|GetHitResultUnderCursorbyChannel "TraceTypeQuery1" true))
  (bind _steerpawn (Variables|Default|GetSteerPawn))
  (bind (_bblockinghit _binitialoverlap _time _distance _location _impactpoint _normal _impactnormal _physmat _hitactor) (Collision|BreakHitResult _hitresult))
  ;[1 1 1] Click Input Player Control
  (:Pressed
    (bind _aspawn (Utilities|Casting|CastToPawn _hitactor)
      (:then
        (if (!= _aspawn _steerpawn)
          (Class|SteerPawn|Evasion _steerpawn _aspawn)
          (Development|PrintString "Evasion")
          (else
            (Class|SteerPawn|Flee _steerpawn (Math|Vector|MakeVector (.x _location) (.y _location) (.z (Transformation|GetActorLocation (Variables|Default|GetSteerPawn)))) :!label _label)
            (Development|PrintString "Flee"))))
      (:CastFailed
        (goto _label)))))

(event Input|KeyboardEvents|LeftShift
  (params (Key :type Key%20Structure :default "None"))
  ;[1 1 1] Click Input Player Control
  (:Pressed
    (Variables|Default|SetisShiftPress true))
  (:Released
    (Variables|Default|SetisShiftPress false)))

(event Input|KeyboardEvents|E
  (params (Key :type Key%20Structure :default "None"))
  ;[1 1 1] CircuitPawn control
  (:Pressed
    (Class|SteerPawn|TwoWay (Variables|Default|GetCircuitPawn))
    (Development|PrintString "Two Way")))

(fn ConstructionScript)
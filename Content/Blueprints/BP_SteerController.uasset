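; Player controller for a steering-behavior pawn, issuing movement commands to the possessed SteerPawn from mouse clicks.
; BeginPlay caches player pawn 0 as SteerPawn, and clicks trace under the cursor on the Visibility channel.
; Left click calls Pursuit on another pawn or Seek to the clicked point, while right click calls Evasion or Flee likewise.
; Target points keep the pawn's own Z, and each command prints its name.
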(event EventBeginPlay
  (bind _assteer_pawn (Utilities|Casting|CastToSteerPawn (Game|Player|GetPlayerPawn 0)))
  (Variables|Default|SetSteerPawn _assteer_pawn))

(event EventTick
  (params (DeltaSeconds :type Float%20%28single-precision%29)))

(event Input|MouseEvents|LeftMouseButton
  (params (Key :type Key%20Structure :default "None"))
  (bind _hitresult (Game|Player|GetHitResultUnderCursorbyChannel "TraceTypeQuery1" true))
  (bind _steerpawn (Variables|Default|GetSteerPawn))
  (bind (_bblockinghit _binitialoverlap _time _distance _location _impactpoint _normal _impactnormal _physmat _hitactor) (Collision|BreakHitResult _hitresult))
  (:Pressed
    (bind _aspawn (Utilities|Casting|CastToPawn _hitactor)
      (:then
        (if (!= _aspawn _steerpawn)
          (Class|SteerPawn|Pursuit _steerpawn _aspawn)
          (Development|PrintString "Pursuit")
          (else
            (Class|SteerPawn|Seek _steerpawn (Math|Vector|MakeVector (.x _location) (.y _location) (.z (Transformation|GetActorLocation (Variables|Default|GetSteerPawn)))) :!label _label)
            (Development|PrintString "Seek"))))
      (:CastFailed
        (goto _label)))))

(event Input|MouseEvents|RightMouseButton
  (params (Key :type Key%20Structure :default "None"))
  (bind _hitresult (Game|Player|GetHitResultUnderCursorbyChannel "TraceTypeQuery1" true))
  (bind _steerpawn (Variables|Default|GetSteerPawn))
  (bind (_bblockinghit _binitialoverlap _time _distance _location _impactpoint _normal _impactnormal _physmat _hitactor) (Collision|BreakHitResult _hitresult))
  (:Pressed
    (bind _aspawn (Utilities|Casting|CastToPawn _hitactor)
      (:then
        (if (!= _aspawn _steerpawn)
          (Class|SteerPawn|Evasion _steerpawn _aspawn)
          (Development|PrintString "Evasion")
          (else
            (Class|SteerPawn|Flee _steerpawn (Math|Vector|MakeVector (.x _location) (.y _location) (.z (Transformation|GetActorLocation (Variables|Default|GetSteerPawn)))) :!label _label)
            (Development|PrintString "Flee"))))
      (:CastFailed
        (goto _label)))))

(fn ConstructionScript)